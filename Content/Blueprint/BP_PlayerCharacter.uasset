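; BP_PlayerCharacter is a player character that moves back and forth along its forward axis from the MoveRight input.
; Only full axis values of at least 1 in either direction act, snapping the mesh yaw to face the travel direction and adding movement input along the actor's forward vector.
; A Camera absolute-rotation call is present but unconnected, and BeginPlay and the construction script are empty.
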(event `self.ReceiveBeginPlay`)

(event `InputAxis|MoveRight`
  (params (AxisValue :type "Float (single-precision)"))
  (bind (_returnvalue_roll _returnvalue_pitch) (`KismetMathLibrary.BreakRotator` (`self.K2_GetActorRotation`)))
  (bind _mesh (`self.Mesh`))
  (if (<= AxisValue -1.0)
    (`SceneComponent.K2_SetRelativeRotation` _mesh (`KismetMathLibrary.MakeRotator` _returnvalue_roll _returnvalue_pitch 90.0) false false)
    (`self.AddMovementInput` (`self.GetActorForwardVector`) AxisValue)
    (elif (>= AxisValue 1.0)
      (`SceneComponent.K2_SetRelativeRotation` _mesh (`KismetMathLibrary.MakeRotator` _returnvalue_roll _returnvalue_pitch -90.0) false false)
      (`self.AddMovementInput` (`self.GetActorForwardVector`) AxisValue))))

(fn `UserConstructionScript`)